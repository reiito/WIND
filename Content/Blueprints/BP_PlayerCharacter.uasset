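; Player character that moves automatically along negative Y while the mouse tilts an umbrella, until it hits an obstacle.
; Clamped mouse X, offset by MaxX, sets UmbrellaPivot pitch; the clamped Y value is computed but unused.
; Overlapping an "Object"-tagged component enables physics on the body and umbrella, stops control and shows the death HUD.
; Once dead, R restarts the level through a console command.
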(event OnComponentBeginOverlap(CapsuleComponent)
  (params (OverlappedComponent :type Primitive%20Component%20Object%20Reference) (OtherActor :type Actor%20Object%20Reference) (OtherComp :type Primitive%20Component%20Object%20Reference) (OtherBodyIndex :type Integer) (bFromSweep :type Boolean) (SweepResult :type Hit%20Result%20Structure%20%28by%20ref%29))
  (if (Components|ComponentHasTag OtherComp "Object")
    (Physics|SetSimulatePhysics (Variables|Character|GetMesh) true)
    (Variables|Default|SetDead true)
    (Variables|Default|SetDeathHUD "Visible")))

(event EventTick
  (params (DeltaSeconds :type Float%20%28single-precision%29))
  (if (not (Variables|Default|GetDead))
    (Pawn|Input|AddMovementInput "0,-5.000000, 0" DeltaSeconds false)))

(event Input|MouseEvents|MouseX
  (params (AxisValue :type Float%20%28single-precision%29))
  (bind _x (CallFunction|CustomXLocation))
  (if (not (Variables|Default|GetDead))
    (Transformation|SetRelativeRotation (Variables|Default|GetUmbrellaPivot) (Math|Rotator|MakeRotator 0.0 (* _x -1.0) 0.0) false false)))

(event Input|MouseEvents|MouseY
  (params (AxisValue :type Float%20%28single-precision%29))
  (CallFunction|CustomYLocation)
  (if (not (Variables|Default|GetDead))
    (Transformation|SetRelativeRotation (Variables|Default|GetUmbrellaPivot) (Math|Rotator|MakeRotator 0.0 (* (stale Input|MouseEvents|MouseX _x) -1.0) 0.0) false false)))

(event Input|KeyboardEvents|R
  (params (Key :type Key%20Structure))
  (:Pressed
    (if (Variables|Default|GetDead)
      (Development|ExecuteConsoleCommand "RestartLevel" 0))))

(fn ConstructionScript)

(fn CustomXLocation
  (bind _maxx (Variables|Default|GetMaxX))
  (return (Math|Float|Clamp(Float) (- (.LocationX (Game|Player|GetMousePosition (Game|GetPlayerController 0))) _maxx) (* _maxx -1.0) _maxx)))

(fn CustomYLocation
  (bind _maxy (Variables|Default|GetMaxY))
  (bind _result (Math|Float|NegateFloat (- (.LocationY (Game|Player|GetMousePosition (Game|GetPlayerController 0))) (.x _maxy)))
    (:%20%20
      (return (Math|Float|Clamp(Float) _result (.y _maxy) (.x _maxy))))))